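; BP_ItemBase is a base item Blueprint that shows an interaction prompt widget to a player in range.
; On range entry it creates the widget for that player's controller, unless one already exists, and adds it to the viewport.
; On range exit it removes the widget, clears the reference and forces garbage collection.
; The file does no range detection itself, as its overlap and tick events are empty.
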(event `/Game/Interaction/InteractionInterface.OnInteractionRangeEntered`
  (params (Player :type "/Game/ThirdPerson/Blueprints/BP_ThirdPersonCharacter Object Reference"))
  (`self.InteractionWidget`
    (:`then`)
    (:`else`
      (bind _returnvalue (`|CreateWidget` "/Game/Interaction/Widgets/Interaction_Widget.Interaction_Widget_C" (cast `PlayerController` (`Pawn.GetController` Player) :!pure true)))
      (bind _output_get (set `self.InteractionWidget` _returnvalue))
      (`UserWidget.AddToViewport` _output_get 0))))

(event `/Game/Interaction/InteractionInterface.OnInteractionRangeExited`
  (bind _interactionwidget (`self.InteractionWidget`)
    (:`then`
      (`Widget.RemoveFromParent` _interactionwidget)
      (set `self.InteractionWidget` null)
      (`KismetSystemLibrary.CollectGarbage`))
    (:`else`)))

(fn `UserConstructionScript`)